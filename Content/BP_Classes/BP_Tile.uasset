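; BP_Tile is a map tile actor, apparently hex-based, that shows its terrain elevation and highlight state.
; UpdateVisuals selects a color-coded TileMesh material from Elevation, running from water through flat ground to three mountain heights.
; It applies a pulsing hex overlay material when IsHighlighted is set and clears it otherwise.
; A switch on Water has only empty branches, and the construction script is empty.
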(event `self.UpdateVisuals`
  (switch `EElevationLevel` "Water"
    (:`Water`
      _)
    (:`Flat`
      _)
    (:`MountainLow`
      _)
    (:`MountainMid`
      _)
    (:`MountainHigh`
      _))
  (`PrimitiveComponent.SetMaterial` (`self.TileMesh`) 0 (select `EElevationLevel` (`self.Elevation`) :`Water` "/Game/MaterialMesh/0_Blue.0_Blue" :`Flat` "/Game/MaterialMesh/1_Green.1_Green" :`MountainLow` "/Game/MaterialMesh/2_Yellow.2_Yellow" :`MountainMid` "/Game/MaterialMesh/3_Orange.3_Orange" :`MountainHigh` "/Game/MaterialMesh/4_Red.4_Red" :!type "MaterialInterface Object Reference"))
  (if (`self.bIsHighlighted`)
    (`MeshComponent.SetOverlayMaterial` (`self.TileMesh`) "/Game/StarterContent/Materials/M_Tech_Hex_Tile_Pulse.M_Tech_Hex_Tile_Pulse")
    (else
      (`MeshComponent.SetOverlayMaterial` (`self.TileMesh`) null))))

(fn `UserConstructionScript`)